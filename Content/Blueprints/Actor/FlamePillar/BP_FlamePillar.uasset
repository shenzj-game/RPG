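; BP_FlamePillar is a flame pillar actor that randomly varies the intensity of its FireLight.
; From BeginPlay, ChoseTImeline randomly picks one of two timelines, and each calls it again on finishing, forming an endless loop.
; The first timeline scales BaseIntensity by its FlameIntensity track.
; The second multiplies BaseIntensity by a constant zero instead of its track, so the light stays dark while it plays.
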(event Custom|StartTimeline_1
  (bind _flameintensity (Timeline|FlameIntensity_1 PlayFromStart)
    (:Update
      (Rendering|Components|Light|SetIntensity (Variables|Default|GetFireLight) (* _flameintensity (Variables|Default|GetBaseIntensity))))
    (:Finished
      (CallFunction|ChoseTImeline))))

(event Custom|StartTimeline_2
  (Timeline|FlameIntensity_2 PlayFromStart
    (:Update
      (Rendering|Components|Light|SetIntensity (Variables|Default|GetFireLight) (* 0.0 (Variables|Default|GetBaseIntensity))))
    (:Finished
      (CallFunction|ChoseTImeline))))

(event Custom|ChoseTImeline
  (switch int (Math|Random|RandomIntegerinRange 0 1)
    (:Default
      (CallFunction|StartTimeline2 :!label _label))
    (:0
      (CallFunction|StartTimeline1))
    (:1
      (goto _label))))

(event EventBeginPlay
  (CallFunction|ChoseTImeline))

(fn ConstructionScript)