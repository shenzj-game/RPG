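; BP_FireBall is a Fire Blast projectile actor that flies out and returns to explode for radial damage.
; On the server, one timeline moves it forward to an apex, then a second lerps it toward ReturnToActor's current location.
; Within explode distance, it calls OnHit, applies radial damage, knockback and death impulse to nearby live players except its owner through Ability System damage params, then destroys itself.
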(event EventBeginPlay)

(event Collision|EventActorBeginOverlap
  (params (OtherActor :type Actor%20Object%20Reference)))

(event EventTick
  (params (DeltaSeconds :type Float%20%28single-precision%29)))

(event EventStartOutgoingTimeline
  (bind _returnvalue (Components|GetOwner))
  (bind _array (Utilities|Array|MakeArray _returnvalue))
  (Networking|SwitchHasAuthority
    (:Authority
      (Variables|Default|SetInitialLocation (Transformation|GetActorLocation))
      (Variables|Default|SetApexLocation (+ (Variables|Default|GetInitialLocation) (* (Transformation|GetActorForwardVector) (Variables|Default|GetTravelDistance))))
      (bind _outgoingtrack (Timeline|OutgoingTimeline Play)
        (:Update
          (Transformation|SetActorLocation (Math|Vector|Lerp(Vector) (Variables|Default|GetInitialLocation) (Variables|Default|GetApexLocation) _outgoingtrack) false false))
        (:Finished
          (bind _returningtrack (Timeline|ReturningTimeline Play)
            (:Update
              (Transformation|SetActorLocation (Math|Vector|Lerp(Vector) (Variables|Default|GetApexLocation) (Transformation|GetActorLocation (Variables|Default|GetReturnToActor)) _returningtrack) false false)
              (if (CallFunction|IsWithinExplodeDistance)
                (Class|RPGProjectile|OnHit)
                (Utilities|Array|Add _array self)
                (bind _outoverlappingactors (Class|RPGAbilitySystemLibrary|GetLivePlayerWithinRadius self _array 3e+02 (Transformation|GetActorLocation)))
                (Variables|Default|SetOverlappingPlayers _outoverlappingactors)
                (Class|RPGAbilitySystemLibrary|SetIsRadialDamageEffectParams (Variables|Default|GetExplosionDamageParams) true 5e+01 3e+02 (Transformation|GetActorLocation))
                (for _array_element (Variables|Default|GetOverlappingPlayers)
                  (Class|RPGAbilitySystemLibrary|SetTargetEffectParamsASC (Variables|Default|GetExplosionDamageParams) (Ability|GetAbilitySystemComponent _array_element))
                  (Class|RPGAbilitySystemLibrary|SetKnockbackDirection (Variables|Default|GetExplosionDamageParams) (- (Transformation|GetActorLocation _array_element) (Transformation|GetActorLocation)) 8e+02)
                  (Class|RPGAbilitySystemLibrary|SetDeathImpulseDirection (Variables|Default|GetExplosionDamageParams) (- (Transformation|GetActorLocation _array_element) (Transformation|GetActorLocation)) 6e+02)
                  (Class|RPGAbilitySystemLibrary|ApplyDamageEffect (Variables|Default|GetExplosionDamageParams)))
                (Actor|DestroyActor)))))))))

(fn ConstructionScript)

(fn IsWithinExplodeDistance
  (return (<= (Math|Vector|VectorLength (- (Transformation|GetActorLocation) (Transformation|GetActorLocation (Variables|Default|GetReturnToActor)))) (Variables|Default|GetExplodeDistance))))